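; Gunslinger is a clickable shooter actor that fires a physics Bullet when clicked and ragdolls when hit.
; Fire spawns the Bullet at its spawn point and launches it along the player's control rotation.
; A capsule hit destroys the capsule and applies an impulse at the nearest physics-asset bone, derived from the other actor's Z velocity.
; The construction script gives gunslingers at high world X a black material, reversed rotation and inverted Impact.
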(event OnClicked(Mesh)
  (params (TouchedComponent :type Primitive%20Component%20Object%20Reference) (ButtonPressed :type Key%20Structure)))

(event OnComponentHit(CapsuleComponent)
  (params (HitComponent :type Primitive%20Component%20Object%20Reference) (OtherActor :type Actor%20Object%20Reference) (OtherComp :type Primitive%20Component%20Object%20Reference) (NormalImpulse :type Vector :default "0, 0, 0") (Hit :type Hit%20Result%20Structure%20%28by%20ref%29))
  (bind _returnvalue (Transformation|GetVelocity OtherActor))
  (bind _returnvalue_2 (Transformation|GetActorLocation OtherActor))
  (bind _z (Math|Vector|BreakVector _returnvalue))
  ;[1 1 1] Impact Collision
  (Components|DestroyComponent (Variables|Collision|GetCapsuleComponent))
  (Physics|SetSimulatePhysics (Variables|Character|GetMesh) true)
  (Physics|AddImpulseatLocation (Variables|Character|GetMesh) (Math|Vector|MakeVector (* _z (Variables|Default|GetImpact)) _z _z) _returnvalue_2 (.BoneName (Class|SkeletalMeshComponent|GetClosestPointonPhysicsAsset (Variables|Character|GetMesh) _returnvalue_2))))

(event MouseInput|EventActorOnClicked
  (params (ButtonPressed :type Key%20Structure))
  (CallFunction|Fire))

(event Input|ActionEvents|InputActionLeftClick
  (params (Key :type Key%20Structure)))

(fn ConstructionScript
  (if (>= (.X (Math|Vector|BreakVector (Transformation|GetActorLocation))) 2e+03)
    (Rendering|Material|SetMaterial (Variables|Character|GetMesh) 0 "/Game/StarterContent/Materials/M_Basic_Wall_black.M_Basic_Wall_black")
    (Transformation|SetActorRotation "0,180.000000, 0")
    (Variables|Default|SetImpact (* (Variables|Default|GetImpact) -1.0))))

(fn Fire
  (bind _returnvalue (Pawn|GetControlRotation :!class /Script/Engine.Pawn))
  (bind _returnvalue_2 (Math|Vector|GetForwardVector _returnvalue))
  (Utilities|Casting|CastToNewPC (Game|GetPlayerController 0))
  (bind _returnvalue_3 (Game|SpawnActorfromClass "/Game/Blueprints/Bullet.Bullet_C" (Math|Transform|MakeTransform (+ (Transformation|GetWorldLocation (Variables|Default|GetProjectileSpawnLocation)) _returnvalue_2) (Transformation|GetWorldRotation (Variables|Collision|GetCapsuleComponent))) "Undefined" 0 (stale _asgunslinger)))
  (Physics|AddImpulse (Variables|/Game/Blueprints/Bullet.Bullet_C|GetStaticMesh _returnvalue_3) (* _returnvalue_2 (Variables|Default|GetShootAmount)) "None" true))