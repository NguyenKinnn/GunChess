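; NewPC is a player controller that shows the mouse cursor when play begins.
; Unconnected node chains would cache the first Grid actor as a Chessboard, pass the visibility-trace hit location under the cursor to its Click, and fire a Gunslinger.
; None of those chains has a triggering event, so only the cursor setting takes effect.
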(event `self.ReceiveBeginPlay`
  (set `self.bShowMouseCursor` true))

(event `InputAction|LeftClick`
  (params (Key :type "Key Structure")))

(event `InputAction|RightClick`
  (params (Key :type "Key Structure")))

(fn `UserConstructionScript`)